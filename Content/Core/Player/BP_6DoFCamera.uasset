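; BP_6DoFCamera is the player's starship camera, turning input into flight, sensor and hyperdrive control with audio feedback.
; Axis inputs adjust flight characteristics, hyperdrive target and HUD opacity, while toggles drive ship and helm sensors.
; Sensor pitch and yaw rotate SensorView through timeline ease-in and ease-out, chained by gates and DoOnce nodes.
; It also opens a port-view window on BeginPlay, sends Jump state over OSC to a panel LED and offers debug message keys.
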(event `Key|RightBracket`
  (params (Key :type "Key Structure"))
  ;[0 0 1] UI Transparency Audio
  (:`Pressed`
    (`GameplayStatics.SpawnSoundAttached` "/Game/ExtendedContent/Sound/SoundFiles/InterfaceSounds/UI_Beep_Double_Clean_Up_stereo.UI_Beep_Double_Clean_Up_stereo" (`self.Root`) "None" (0.0 0.0 0.0) (struct) "KeepRelativeOffset" false 1.0 1.0 0.0 null null)))

(event `Key|LeftBracket`
  (params (Key :type "Key Structure"))
  ;[0 0 1] UI Transparency Audio
  (:`Pressed`
    (`GameplayStatics.SpawnSoundAttached` "/Game/ExtendedContent/Sound/SoundFiles/InterfaceSounds/UI_Beep_Double_Clean_Down_stereo.UI_Beep_Double_Clean_Down_stereo" (`self.Root`) "None" (0.0 0.0 0.0) (struct) "KeepRelativeOffset" false 1.0 1.0 0.0 null null)))

(event `InputAxis|UITransparency`
  (params (AxisValue :type "Float (single-precision)"))
  ;[1 1 1] Adjust UI Opacity
  (`/GeneralFrameworkPlugin/Core/Global/Utils/GeneralExtendedMacroLib.HandleSinglePressAxisButton` AxisValue)
  (message `/Game/Core/Interfaces/I_HUDHandler.UpdateUITransparency` (`PlayerController.GetHUD` (`GameplayStatics.GetPlayerController` 0)) (`KismetMathLibrary.FClamp` AxisValue -1.0)))

(event `Key|AnyKey`
  (params (Key :type "Key Structure"))
  ;[1 1 1] Display Any Key Pressed
  (:`Pressed`
    (`/GeneralFrameworkPlugin/Core/Global/Utils/GeneralHelperLib.Write Debug Message` (`KismetStringLibrary.Concat_StrStr` "PressedKey:" (`KismetTextLibrary.Conv_TextToString` (`KismetInputLibrary.Key_GetDisplayName` Key))) (struct :`R` 1.0 :`B` 0.005385 :`A` 1.0) true 10.0)))

(event `Key|BackSpace`
  (params (Key :type "Key Structure"))
  (bind _root (`self.Root`))
  ;[1 1 1] Enable Screen Messages
  (:`Pressed`
    (`/Engine/EditorBlueprintResources/StandardMacros.FlipFlop`
      (:`A`
        (`KismetSystemLibrary.ExecuteConsoleCommand` "ENABLEALLSCREENMESSAGES" null)
        (`GameplayStatics.SpawnSoundAttached` "/Game/ExtendedContent/Sound/SoundFiles/InterfaceSounds/UI_Toggle_Voice_Tripe_Note_Enable_stereo.UI_Toggle_Voice_Tripe_Note_Enable_stereo" _root "None" (0.0 0.0 0.0) (struct) "KeepRelativeOffset" false 1.0 1.0 0.0 null null))
      (:`B`
        (`KismetSystemLibrary.ExecuteConsoleCommand` "DISABLEALLSCREENMESSAGES" null)
        (`GameplayStatics.SpawnSoundAttached` "/Game/ExtendedContent/Sound/SoundFiles/InterfaceSounds/UI_Toggle_Voice_Triple_Note_Disable_stereo.UI_Toggle_Voice_Triple_Note_Disable_stereo" _root "None" (0.0 0.0 0.0) (struct) "KeepRelativeOffset" false 1.0 1.0 0.0 null null)))))

(event `self.ReceiveBeginPlay`
  (`parent.ReceiveBeginPlay`)
  (`TimelineComponent.SetPlayRate` (`self.EaseOut`) (/ 1.0 (`self.SensorEaseOutInSpeed`)))
  (`TimelineComponent.SetPlayRate` (`self.EaseIn`) (/ 1.0 (`self.SensorEaseOutInSpeed`)))
  (`/QubitStarship/StarshipSystem/Components/StarshipMovementComp.Apply Starship Movement` (`self.StarshipMovementComp`) 1.0 "NewEnumerator0")
  (if true :!pinned true
    (bind _returnvalue (`|CreateWidget` "/Game/UserInterface/Widgets/WB_PortView.WB_PortView_C"))
    (`MultiWindowBPLibrary.CreateMultiWindow` _returnvalue (0.0 0.0) (500.0 500.0) true)))

(event `InputAction|Jump`
  (params (Key :type "Key Structure"))
  ;[1 1 1] Enable OSC Communication
  (:`Pressed`
    (set `self.PanelLEDState` 1)
    (message `/OSCMessaging/I_OSCHandler.SendOSCMessage` (`/OSCMessaging/OSCLib.GetOSCHandler`) "/led" (`|MakeMap` 0 (`self.PanelLEDState`)) :!label _label))
  (:`Released`
    (set `self.PanelLEDState` 0)
    (goto _label)))

(event `InputAxis|ThrustLevel`
  (params (AxisValue :type "Float (single-precision)"))
  ;[1 1 1] Flight Characteristics
  (`/GeneralFrameworkPlugin/Core/Global/Utils/GeneralExtendedMacroLib.HandleSinglePressAxisButton` AxisValue)
  (`/QubitStarship/StarshipSystem/FlightLib.UpdateStarshipFlightCharacteristics` self "NewEnumerator0" (`KismetMathLibrary.FTrunc` (`KismetMathLibrary.FClamp` AxisValue -1.0))))

(event `Key|HIDJoystick_DPADUP`
  (params (Key :type "Key Structure"))
  ;[0 0 1] Flight Characteristics Interface Audio
  (:`Pressed`
    (`GameplayStatics.SpawnSoundAttached` "/Game/ExtendedContent/Sound/SoundFiles/InterfaceSounds/UI_Animate_Stutter_Beep_Appear_stereo.UI_Animate_Stutter_Beep_Appear_stereo" (`self.Root`) "None" (0.0 0.0 0.0) (struct) "KeepRelativeOffset" false 1.0 1.0 0.0 null null :!label _label_2)))

(event `InputAxis|SelectTarget`
  (params (AxisValue :type "Float (single-precision)"))
  ;[1 1 1] Sensor Point Toward Target
  (`/GeneralFrameworkPlugin/Core/Global/Utils/GeneralExtendedMacroLib.HandleSinglePressAxisButton` AxisValue)
  (`/QubitStarship/StarshipSystem/Components/StarshipHyperdriveComp.UpdateTarget` (`self.StarshipHyperdriveComp`) (`KismetMathLibrary.FClamp` AxisValue -1.0))
  (message `/Game/Core/Interfaces/I_HUDHandler.UpdateHUD` (`PlayerController.GetHUD` (`GameplayStatics.GetPlayerController` 0))))

(event `Key|One`
  (params (Key :type "Key Structure"))
  ;[0 0 1] Flight Characteristics Interface Audio
  (:`Pressed`
    (goto _label_2)))

(event `Key|HIDJoystick_DPADRIGHT`
  (params (Key :type "Key Structure"))
  ;[0 0 1] Flight Characteristics Interface Audio
  (:`Pressed`
    (goto _label_2)))

(event `Key|Three`
  (params (Key :type "Key Structure"))
  ;[0 0 1] Flight Characteristics Interface Audio
  (:`Pressed`
    (goto _label_2)))

(event `InputAxis|TurnLevel`
  (params (AxisValue :type "Float (single-precision)"))
  ;[1 1 1] Flight Characteristics
  (`/GeneralFrameworkPlugin/Core/Global/Utils/GeneralExtendedMacroLib.HandleSinglePressAxisButton` AxisValue)
  (`/QubitStarship/StarshipSystem/FlightLib.UpdateStarshipFlightCharacteristics` self "NewEnumerator1" (`KismetMathLibrary.FTrunc` (`KismetMathLibrary.FClamp` AxisValue -1.0))))

(event `Key|Five`
  (params (Key :type "Key Structure"))
  ;[0 0 1] Flight Characteristics Interface Audio
  (:`Pressed`
    (goto _label_2)))

(event `InputAxis|SensorPitch`
  (params (AxisValue :type "Float (single-precision)"))
  ;[1 1 1] Sensor Controlling
  (if (!= AxisValue 0.0)
    (`self.SensorEaseIn`)
    (set `self.LastSensorPitch` AxisValue)
    (else
      (`self.SensorEaseOut`))))

(event `Key|HIDJoystick_DPADDOWN`
  (params (Key :type "Key Structure"))
  ;[0 0 1] Flight Characteristics Interface Audio
  (:`Pressed`
    (`GameplayStatics.SpawnSoundAttached` "/Game/ExtendedContent/Sound/SoundFiles/InterfaceSounds/UI_Animate_Stutter_Beep_Disappear_stereo.UI_Animate_Stutter_Beep_Disappear_stereo" (`self.Root`) "None" (0.0 0.0 0.0) (struct) "KeepRelativeOffset" false 1.0 1.0 0.0 null null :!label _label_3)))

(event `Key|Two`
  (params (Key :type "Key Structure"))
  ;[0 0 1] Flight Characteristics Interface Audio
  (:`Pressed`
    (goto _label_3)))

(event `Key|HIDJoystick_DPADLEFT`
  (params (Key :type "Key Structure"))
  ;[0 0 1] Flight Characteristics Interface Audio
  (:`Pressed`
    (goto _label_3)))

(event `InputAxis|DamperLevel`
  (params (AxisValue :type "Float (single-precision)"))
  ;[1 1 1] Flight Characteristics
  (`/GeneralFrameworkPlugin/Core/Global/Utils/GeneralExtendedMacroLib.HandleSinglePressAxisButton` AxisValue)
  (`/QubitStarship/StarshipSystem/FlightLib.UpdateStarshipFlightCharacteristics` self "NewEnumerator2" (`KismetMathLibrary.FTrunc` (`KismetMathLibrary.FClamp` AxisValue -1.0))))

(event `Key|Four`
  (params (Key :type "Key Structure"))
  ;[0 0 1] Flight Characteristics Interface Audio
  (:`Pressed`
    (goto _label_3)))

(event `Key|Backslash`
  (params (Key :type "Key Structure")))

(event `Key|Six`
  (params (Key :type "Key Structure"))
  ;[0 0 1] Flight Characteristics Interface Audio
  (:`Pressed`
    (goto _label_3)))

(event `InputAxis|SensorYaw`
  (params (AxisValue :type "Float (single-precision)"))
  ;[1 1 1] Sensor Controlling
  (if (!= AxisValue 0.0)
    (`self.SensorEaseIn`)
    (set `self.LastSensorYaw` AxisValue)
    (else
      (`self.SensorEaseOut`))))

(event `InputAction|ToggleSensor`
  (params (Key :type "Key Structure"))
  (:`Pressed`
    (`/QubitStarship/StarshipSystem/SensorSystem/StarshipSensoric.ToggleSensors` (`self.StarshipSensoric`))
    (bind _returnvalue (`GameplayStatics.GetActorOfClass` "/SkyPosition/Blueprints/BP_SkyPosition.BP_SkyPosition_C"))
    (if (`KismetSystemLibrary.IsValid` _returnvalue)
      (`/SkyPosition/Blueprints/BP_SkyPosition.UpdateSetting` _returnvalue))))

(event `SensorEaseIn`
  (bind _sensorspeed (`self.SensorSpeed`))
  ;[1 1 1] Sensor Controlling
  (`|ExecutionSequence`
    (:`then_0`
      (`/Engine/EditorBlueprintResources/StandardMacros.DoOnce` false :!label _label_4
        (:`Completed`
          (`TimelineComponent.Stop` (`self.EaseOut`))
          (bind (_direction _newtrack_0) (`Timeline|EaseIn` :!via `PlayFromStart`)
            (:`Update`
              (`SceneComponent.K2_AddRelativeRotation` (`self.SensorView`) (`KismetMathLibrary.MakeRotator` 0.0 (* _newtrack_0 (`self.GetInputAxisValue`) _sensorspeed) (* _newtrack_0 (`self.GetInputAxisValue`) _sensorspeed)) false false))
            (:`Finished`
              (`self.OnEaseInFinish`))))))
    (:`then_1`
      (`/Engine/EditorBlueprintResources/StandardMacros.Gate` true :!label _label_5
        (:`Exit`
          (`SceneComponent.K2_AddRelativeRotation` (`self.SensorView`) (`KismetMathLibrary.MakeRotator` 0.0 (* (`self.GetInputAxisValue`) (`self.SensorSpeed`)) (* (`self.GetInputAxisValue`) (`self.SensorSpeed`))) false false))))
    (:`then_2`
      (`self.ResetEaseOut`))))

(event `OnEaseOutFInish`
  ;[1 1 1] Sensor Controlling
  (goto _label_4 :!via `Reset`))

(event `InputAction|ToggleHelmSensor`
  (params (Key :type "Key Structure"))
  (:`Pressed`
    (`/QubitStarship/StarshipSystem/SensorSystem/StarshipSensoric.ToggleSensors` (`self.HelmSensoric`))
    (bind _returnvalue (`GameplayStatics.GetActorOfClass` "/SkyPosition/Blueprints/BP_SkyPosition.BP_SkyPosition_C"))
    (if (`KismetSystemLibrary.IsValid` _returnvalue)
      (`/SkyPosition/Blueprints/BP_SkyPosition.UpdateSetting` _returnvalue))))

(event `OnEaseInFinish`
  ;[1 1 1] Sensor Controlling
  (goto _label_5 :!via `Open`))

(event `OnEaseOutStarted`
  ;[1 1 1] Sensor Controlling
  (goto _label_5 :!via `Close`))

(event `InputAxis|ChangeSensorTarget`
  (params (AxisValue :type "Float (single-precision)"))
  (if (!= AxisValue 0.0)
    (`/QubitStarship/StarshipSystem/SensorSystem/StarshipSensoric.ChangeTarget` (`self.StarshipSensoric`) AxisValue)))

(event `Key|Zero`
  (params (Key :type "Key Structure"))
  ;[0 0 1] Sensors and Hyperdrive Interface Audio
  (:`Pressed`
    (`GameplayStatics.SpawnSoundAttached` "/Game/ExtendedContent/Sound/SoundFiles/InterfaceSounds/UI_Animate_Clean_Beeps_Appear_stereo.UI_Animate_Clean_Beeps_Appear_stereo" (`self.Root`) "None" (0.0 0.0 0.0) (struct) "KeepRelativeOffset" false 1.0 1.0 0.0 null null :!label _label_6)))

(event `Key|B`
  (params (Key :type "Key Structure"))
  ;[0 0 1] Sensors and Hyperdrive Interface Audio
  (:`Pressed`
    (`/Engine/EditorBlueprintResources/StandardMacros.FlipFlop` :!label _label_7
      (:`A`
        (goto _label_6))
      (:`B`
        (`GameplayStatics.SpawnSoundAttached` "/Game/ExtendedContent/Sound/SoundFiles/InterfaceSounds/UI_Animate_Clean_Beeps_Disappear_stereo.UI_Animate_Clean_Beeps_Disappear_stereo" (`self.Root`) "None" (0.0 0.0 0.0) (struct) "KeepRelativeOffset" false 1.0 1.0 0.0 null null :!label _label_8)))))

(event `Key|PageUp`
  (params (Key :type "Key Structure"))
  ;[0 0 1] Sensors and Hyperdrive Interface Audio
  (:`Pressed`
    (goto _label_6)))

(event `SensorEaseOut`
  (bind _sensorspeed (`self.SensorSpeed`))
  ;[1 1 1] Sensor Controlling
  (`/Engine/EditorBlueprintResources/StandardMacros.DoOnce` false :!label _label_9
    (:`Completed`
      (`self.OnEaseOutStarted`)
      (`TimelineComponent.Stop` (`self.EaseIn`))
      (bind (_direction _newtrack_0) (`Timeline|EaseOut` :!via `PlayFromStart`)
        (:`Update`
          (`SceneComponent.K2_AddRelativeRotation` (`self.SensorView`) (`KismetMathLibrary.MakeRotator` 0.0 (* _newtrack_0 (`self.LastSensorPitch`) _sensorspeed) (* _newtrack_0 (`self.LastSensorYaw`) _sensorspeed)) false false))
        (:`Finished`
          (`self.OnEaseOutFInish`)
          (set `self.LastSensorYaw` (`self.GetInputAxisValue`))
          (set `self.LastSensorPitch` (`self.GetInputAxisValue`)))))))

(event `Key|HIDJoystick_Button7`
  (params (Key :type "Key Structure"))
  ;[0 0 1] Sensors and Hyperdrive Interface Audio
  (:`Pressed`
    (goto _label_6)))

(event `Key|HIDJoystick_Button11`
  (params (Key :type "Key Structure"))
  ;[0 0 1] Sensors and Hyperdrive Interface Audio
  (:`Pressed`
    (goto _label_7)))

(event `Key|N`
  (params (Key :type "Key Structure"))
  ;[0 0 1] Sensors and Hyperdrive Interface Audio
  (:`Pressed`
    (goto _label_6)))

(event `InputAxis|ChangeHelmTarget`
  (params (AxisValue :type "Float (single-precision)"))
  (if (!= AxisValue 0.0)
    (`/QubitStarship/StarshipSystem/SensorSystem/StarshipSensoric.ChangeTarget` (`self.HelmSensoric`) AxisValue)))

(event `ResetEaseOut`
  ;[1 1 1] Sensor Controlling
  (goto _label_9 :!via `Reset`))

(event `Key|HIDJoystick_Button9`
  (params (Key :type "Key Structure"))
  ;[0 0 1] Sensors and Hyperdrive Interface Audio
  (:`Pressed`
    (goto _label_8)))

(event `Key|PageDown`
  (params (Key :type "Key Structure"))
  ;[0 0 1] Sensors and Hyperdrive Interface Audio
  (:`Pressed`
    (goto _label_8)))

(event `Key|Nine`
  (params (Key :type "Key Structure"))
  ;[0 0 1] Sensors and Hyperdrive Interface Audio
  (:`Pressed`
    (goto _label_8)))

(event `Key|M`
  (params (Key :type "Key Structure"))
  ;[0 0 1] Sensors and Hyperdrive Interface Audio
  (:`Pressed`
    (goto _label_8)))

(event `InputAction|ToggleHelmSensor`
  (params (Key :type "Key Structure"))
  ;[0 0 1] Sensors and Hyperdrive Interface Audio
  (:`Pressed`
    (goto _label_7)))

(fn `UserConstructionScript`
  (`parent.UserConstructionScript`))