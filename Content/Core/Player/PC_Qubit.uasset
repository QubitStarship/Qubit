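; PC_Qubit is the player controller that runs a hyperdrive jump from the solar system level to Venus.
; The Hyperdrive input plays audio, streams in a transition level and then VenusMap with timed delays, then unloads QubitSolarSystem and the transition level.
; Before unloading, FindNewLocation turns the pawn toward the Venus-tagged planet and teleports it back from the planet by a scale-based distance.
; The destination is hardcoded to Venus, though a comment assigns target selection to a Sensor UI.
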(event `InputAction|Hyperdrive`
  (params (Key :type "Key Structure"))
  (:`Pressed`
    (`/QubitStarship/AudioSystem/AudioSystemComp.PlaySpecificAudio` (`self.AudioSystemComp`) false "Hyperdrive")
    (`GameplayStatics.LoadStreamLevel` "Hyperdrive" true true)
    (`KismetSystemLibrary.Delay` 1.0)
    (`GameplayStatics.LoadStreamLevel` "VenusMap" true true)
    (`KismetSystemLibrary.Delay` 2.0)
    (`self.FindNewLocation`)
    (`GameplayStatics.UnloadStreamLevel` "QubitSolarSystem" true)
    (`GameplayStatics.UnloadStreamLevel` "Hyperdrive" true)
    (`self.SetViewTargetWithBlend` (`self.K2_GetPawn`))
    (`/QubitStarship/AudioSystem/AudioSystemComp.StopAudio` (`self.AudioSystemComp`) true 3.0)))

(fn `FindNewLocation`
  (bind _returnvalue (`self.K2_GetPawn`))
  ;[1 1 1] Target Location _> determined by Sensor UI
  (bind _outactors (`GameplayStatics.GetAllActorsOfClassWithTag` "/QubitStarship/PlanetarySystem/BP_PlanetMASTER.BP_PlanetMASTER_C" "Venus"))
  (bind _output (`|GetArrayItem` _outactors))
  (bind _returnvalue_2 (`self.K2_GetActorLocation` _output))
  (`self.K2_SetActorRotation` _returnvalue (`KismetMathLibrary.FindLookAtRotation` (`self.K2_GetActorLocation` _returnvalue) _returnvalue_2) false)
  (bind _returnvalue_x (`KismetMathLibrary.BreakVector` (`self.GetActorScale3D` _output)))
  (set `self.TargetLocation` (+ _returnvalue_2 (* (`self.GetActorForwardVector` _returnvalue) -1000.0 _returnvalue_x)))
  (`self.K2_SetActorLocation` (`self.K2_GetPawn`) (`self.TargetLocation`) false true))

(fn `UserConstructionScript`)